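; Level game mode that serves as a hub for tutorial display, pickup sound effects and background music.
; On BeginPlay it caches the player's LevelHUD and, only if that cast succeeds, creates an AudioComponent at the world origin.
; Tutorial events show or hide keyed tutorials through the HUD, and points and orbs events play one-shot sounds at the origin.
; PlayMusic switches that component between menu and level tracks, and StopMusic halts it.
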(event EventEnterTutorialEvent
  (params (Key :type String))
  ;[1 1 1] Tutorial
  (Default|ShowTutorial (Variables|Default|GetHUD) Key))

(event EventPointsSoundEvent
  ;[1 1 1] SOUNDS
  ;;[1 1 1] Points
  (Audio|PlaySoundatLocation 0 "/Game/Sounds/CoinEffect16bit.CoinEffect16bit"))

(event EventOrbsSoundEvent
  ;[1 1 1] SOUNDS
  ;;[1 1 1] Orbs
  (Audio|PlaySoundatLocation 0 "/Game/Sounds/OrbEffect16bit.OrbEffect16bit"))

(event EventExitTutorialEvent
  ;[1 1 1] Tutorial
  (Default|HideTutorial (Variables|Default|GetHUD)))

(event EventBeginPlay
  (bind _aslevel_hud (Utilities|Casting|CastToLevelHUD (HUD|GetHUD (Game|GetPlayerController 0))))
  (Variables|Default|SetHUD _aslevel_hud)
  (bind _returnvalue (AddComponent|AddAudioComponent false))
  (bind _output_get (Variables|Default|SetaudioComponent _returnvalue))
  (Transformation|SetWorldLocation _output_get "0, 0, 0" false))

(fn ConstructionScript)

(fn PlayMusic
  (params (isMenuTrack :type Boolean :default false))
  (bind _audiocomponent (Variables|Default|GetaudioComponent))
  (if isMenuTrack
    (Audio|Components|Audio|SetSound _audiocomponent "/Game/Sounds/Menu_track.Menu_track")
    (else
      (Audio|Components|Audio|SetSound _audiocomponent "/Game/Sounds/LevelTrack01_16bit.LevelTrack01_16bit")))
  (Audio|Components|Audio|Play _audiocomponent 0.0))

(fn StopMusic
  (Audio|Components|Audio|Stop (Variables|Default|GetaudioComponent)))