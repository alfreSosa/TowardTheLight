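; MyGameModeBP is a game mode Blueprint that provides sound effect playback for points and orbs.
; On BeginPlay it adds two audio components at runtime, AudioPoints and AudioOrbs, and assigns them the 16-bit coin and orb sounds.
; The custom events PointsSoundEvent and OrbsSoundEvent each play their component from the start, then move it to the world origin.
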(event EventPointsSoundEvent
  (bind _audiopoints (Variables|Default|GetaudioPoints))
  ;[1 1 1] Points
  (Audio|Components|Audio|Play _audiopoints 0.0)
  (Transformation|SetWorldLocation _audiopoints "0, 0, 0" false))

(event EventOrbsSoundEvent
  (bind _audioorbs (Variables|Default|GetaudioOrbs))
  ;[1 1 1] Orbs
  (Audio|Components|Audio|Play _audioorbs 0.0)
  (Transformation|SetWorldLocation _audioorbs "0, 0, 0" false))

(event EventBeginPlay
  ;[1 1 1] Init
  (bind _returnvalue (AddComponent|AddAudioComponent false))
  (Variables|Default|SetaudioPoints _returnvalue)
  (bind _returnvalue_2 (AddComponent|AddAudioComponent false))
  (Variables|Default|SetaudioOrbs _returnvalue_2)
  (Audio|Components|Audio|SetSound (Variables|Default|GetaudioPoints) "/Game/Sounds/CoinEffect16bit.CoinEffect16bit")
  (Audio|Components|Audio|SetSound (Variables|Default|GetaudioOrbs) "/Game/Sounds/OrbEffect16bit.OrbEffect16bit"))

(fn ConstructionScript)